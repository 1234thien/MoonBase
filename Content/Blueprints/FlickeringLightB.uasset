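; Flickering spotlight fixture actor whose construction script applies exposed color, intensity, cone, shape and rotation settings to the light.
; When Flicker is set, BeginPlay waits a random delay, then randomly plays or reverses an intensity timeline, with playback completion looping back to the delay.
; Timeline updates scale the spotlight intensity and swap the mesh material to dark below half intensity or at zero, otherwise lit.
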(event EventBeginPlay
  (bind _intensity (Variables|Default|GetIntensity))
  (bind _sm_light_b (Variables|Default|GetSM_Light_B))
  (if (Variables|Default|GetFlicker)
    (Utilities|FlowControl|Delay (+ (Math|Random|RandomFloat) (Math|Random|RandomFloat)) :!label _label)
    (if (Math|Random|RandomBool)
      (bind _intensity_2 (Timeline|Timeline_0 Play)
        (:Update
          (Rendering|Components|Light|SetIntensity (Variables|Default|GetSpotLight) (* _intensity_2 _intensity))
          (if (or (> (/ _intensity 2.0) (* _intensity_2 _intensity)) (== _intensity 0.0))
            (Rendering|Material|SetMaterial _sm_light_b 1 (Variables|Default|GetDarkMat))
            (else
              (Rendering|Material|SetMaterial _sm_light_b 1 (Variables|Default|GetLightMat)))))
        (:Finished
          (goto _label)))
      (elif (Math|Random|RandomBool)
        (Timeline|Timeline_0 PlayFromStart)
        (elif (Math|Random|RandomBool)
          (Timeline|Timeline_0 Reverse)
          (else
            (Timeline|Timeline_0 ReverseFromEnd)))))))

(event Collision|EventActorBeginOverlap
  (params (OtherActor :type Actor%20Object%20Reference)))

(event EventTick
  (params (DeltaSeconds :type Float%20%28single-precision%29)))

(fn ConstructionScript
  (bind _spotlight (Variables|Default|GetSpotLight))
  (Rendering|Components|Light|SetLightColor _spotlight (Math|Conversions|ToLinearColor(Color) (Variables|Default|GetColor)) true)
  (Rendering|Components|Light|SetIntensity _spotlight (Variables|Default|GetIntensity))
  (Rendering|Lighting|SetOuterConeAngle _spotlight (Variables|Default|GetOuter%20Cone%20Angle))
  (Rendering|Lighting|SetAttenuationRadius _spotlight (Variables|Default|GetAttenuation%20Radius))
  (Class|PointLightComponent|SetSourceRadius _spotlight (Variables|Default|GetSource%20Radius))
  (Rendering|Lighting|SetInnerConeAngle _spotlight (Variables|Default|GetInner%20Cone%20Angle))
  (Class|PointLightComponent|SetSourceLength _spotlight (Variables|Default|GetSource%20Length))
  (Transformation|SetRelativeRotation _spotlight (Variables|Default|GetRotation) false false)
  (Rendering|Material|SetMaterial (Variables|Default|GetSM_Light_B) 1 (Variables|Default|GetLightMat)))