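; A spotlight fixture actor that can flicker at random intervals when its Flicker option is on.
; The construction script applies the exposed color, intensity, cone angle and attenuation radius to the spotlight.
; At play start, a random delay triggers the Flickering timeline in a randomly chosen playback mode, and timeline completion restarts the cycle.
; The timeline scales intensity and swaps a mesh material between lit and dark around half brightness.
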(event EventBeginPlay
  (bind _intensity (Variables|Default|GetIntensity))
  (bind _sm_light_a (Variables|Default|GetSM_Light_A))
  (bind _returnvalue (/ _intensity 2.0))
  (if (Variables|Default|GetFlicker)
    (Utilities|FlowControl|Delay (+ (Math|Random|RandomFloat) (Math|Random|RandomFloat)) :!label _label)
    (if (Math|Random|RandomBool)
      (bind _intensity_2 (Timeline|Flickering Play)
        (:Update
          (Rendering|Components|Light|SetIntensity (Variables|Default|GetSpotLight) (* _intensity_2 _intensity))
          (if (or (> _returnvalue (* _intensity_2 _intensity)) (== 0.0 _returnvalue))
            (Rendering|Material|SetMaterial _sm_light_a 2 (Variables|Default|GetDarkMat))
            (else
              (Rendering|Material|SetMaterial _sm_light_a 2 (Variables|Default|GetLightMat)))))
        (:Finished
          (goto _label)))
      (elif (Math|Random|RandomBool)
        (Timeline|Flickering PlayFromStart)
        (elif (Math|Random|RandomBool)
          (Timeline|Flickering Reverse)
          (else
            (Timeline|Flickering ReverseFromEnd)))))))

(event Collision|EventActorBeginOverlap
  (params (OtherActor :type Actor%20Object%20Reference)))

(event EventTick
  (params (DeltaSeconds :type Float%20%28single-precision%29)))

(fn ConstructionScript
  (bind _spotlight (Variables|Default|GetSpotLight))
  (Rendering|Components|Light|SetLightColor _spotlight (Math|Conversions|ToLinearColor(Color) (Variables|Default|GetColor)) true)
  (Rendering|Components|Light|SetIntensity _spotlight (Variables|Default|GetIntensity))
  (Rendering|Lighting|SetOuterConeAngle _spotlight (Variables|Default|GetOuter%20Cone%20Angle))
  (Rendering|Lighting|SetAttenuationRadius _spotlight (Variables|Default|GetAttenuation%20Radius)))