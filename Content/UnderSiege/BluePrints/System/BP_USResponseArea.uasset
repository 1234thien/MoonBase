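; BP_USResponseArea is a trigger-sphere zone that supplies nearby turrets with a list of enemy targets.
; On BeginPlay it finds tagged turrets within TriggerSphereRadius and casts to the five turret classes to hand each a reference to itself.
; Tick rebuilds the target array from overlapping enemy-tagged actors, throttled to half-second intervals by a delay-reset flag.
; The construction script uses the same radius value as the sphere's world scale.
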(event EventBeginPlay
  (bind _self self)
  (bind _outactors (Actor|GetAllActorswithTag "USTurretArhetype"))
  (for _array_element _outactors
    (if (<= (Transformation|GetDistanceTo self _array_element) (Variables|USControl|GetTriggerSphereRadius))
      (bind _asbp_usturret_1 (Utilities|Casting|CastToBP_USTurret1 _array_element)
        (:then
          (Variables|/Game/UnderSiege/BluePrints/Turret/BP_USTurret1.BP_USTurret1_C|SetUSResponseAreaRef _asbp_usturret_1 _self))
        (:CastFailed
          _))
      (bind _asbp_usturret_2 (Utilities|Casting|CastToBP_USTurret2 _array_element)
        (:then
          (Variables|/Game/UnderSiege/BluePrints/Turret/BP_USTurret2.BP_USTurret2_C|SetUSResponseAreaRef _asbp_usturret_2 _self))
        (:CastFailed
          _))
      (bind _asbp_usturret_3 (Utilities|Casting|CastToBP_USTurret3 _array_element)
        (:then
          (Variables|/Game/UnderSiege/BluePrints/Turret/BP_USTurret3.BP_USTurret3_C|SetUSResponseAreaRef _asbp_usturret_3 _self))
        (:CastFailed
          _))
      (bind _asbp_usturret_4 (Utilities|Casting|CastToBP_USTurret4 _array_element)
        (:then
          (Variables|/Game/UnderSiege/BluePrints/Turret/BP_USTurret4.BP_USTurret4_C|SetUSResponseAreaRef _asbp_usturret_4 _self))
        (:CastFailed
          _))
      (bind _asbp_usturret_5 (Utilities|Casting|CastToBP_USTurret5 _array_element))
      (Variables|/Game/UnderSiege/BluePrints/Turret/BP_USTurret5.BP_USTurret5_C|SetUSResponseAreaRef _asbp_usturret_5 _self))))

(event EventTick
  (params (DeltaSeconds :type Float%20%28single-precision%29))
  (if (not (Variables|Default|GetTargetsTimeout))
    (Utilities|Array|Clear (Variables|Default|GetUSResponseAreaTargets))
    (for _array_element (Collision|GetOverlappingActors (Variables|Default|GetTriggerSphere) 0 :!class /Script/Engine.PrimitiveComponent)
      (if (Actor|ActorHasTag _array_element "USEnemyArhetype")
        (Utilities|Array|Add (Variables|Default|GetUSResponseAreaTargets) _array_element)))
    (Variables|Default|SetTargetsTimeout true)
    (Utilities|FlowControl|Delay 0.5)
    (Variables|Default|SetTargetsTimeout false)))

(fn ConstructionScript
  (bind _triggersphereradius (Variables|USControl|GetTriggerSphereRadius))
  (Transformation|SetWorldScale3D (Variables|Default|GetTriggerSphere) (Math|Vector|MakeVector _triggersphereradius _triggersphereradius _triggersphereradius)))