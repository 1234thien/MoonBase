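; BP_USTurret1 is a floor or inverted (DownTurret) turret that shoots BP_USBullet1 at actors in its linked response area.
; Tick picks a random target, plays the shield animation, then after a ready delay engages only targets above it, or below when inverted.
; Base yaw and gun pitch interpolate toward the target while Delay paces shots and emissive glow builds.
; Without a target, the glow fades and the shield animation reverses.
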(event EventBeginPlay
  (bind _defaultsceneroot (Variables|Default|GetDefaultSceneRoot))
  (Rendering|Material|CreateDynamicMaterialInstance (Variables|Default|GetSM_turret1_gun) 0 0 "None" :!class /Script/Engine.PrimitiveComponent)
  (if (Variables|USControl|GetDownTurret)
    (Transformation|SetWorldRotation _defaultsceneroot "180.000000,180.000000,180.000000" false false)
    (Transformation|SetWorldRotation (Variables|Default|GetSM_turret1_base) "180.000000,0.000000,0.000000" false false)
    (else
      (Transformation|SetWorldRotation _defaultsceneroot "0, 0, 0" false false))))

(event EventTick
  (params (DeltaSeconds :type Float%20%28single-precision%29))
  (bind _sm_turret1_gun (Variables|Default|GetSM_turret1_gun))
  (bind _downturret (Variables|USControl|GetDownTurret))
  (bind _turret1_shield (Variables|Default|Getturret1_shield))
  (bind _turret1_shield_2 (Variables|Default|Getturret1_shield))
  (bind _sm_turret1_gun_2 (Variables|Default|GetSM_turret1_gun))
  (bind _sm_turret1_gun_3 (Variables|Default|GetSM_turret1_gun))
  (bind _returnvalue (Transformation|GetWorldLocation _sm_turret1_gun_3))
  (bind _usresponsearearef (Variables|USControl|GetUSResponseAreaRef)
    (:then
      (if (Variables|Default|GetIsAim)
        (if (Utilities|IsValid (Utilities|Array|Get(acopy) (Variables|/Game/UnderSiege/BluePrints/System/BP_USResponseArea.BP_USResponseArea_C|GetUSResponseAreaTargets _usresponsearearef) (Variables|Default|GetTargetOffset)))
          (if (Variables|Default|GetIsReady)
            (if (or (and (not (Variables|USControl|GetDownTurret)) (> (.z (Transformation|GetActorLocation (Utilities|Array|Get(acopy) (Variables|/Game/UnderSiege/BluePrints/System/BP_USResponseArea.BP_USResponseArea_C|GetUSResponseAreaTargets _usresponsearearef) (Variables|Default|GetTargetOffset)))) (.z (Transformation|GetActorLocation)))) (and (Variables|USControl|GetDownTurret) (< (.z (Transformation|GetActorLocation (Utilities|Array|Get(acopy) (Variables|/Game/UnderSiege/BluePrints/System/BP_USResponseArea.BP_USResponseArea_C|GetUSResponseAreaTargets _usresponsearearef) (Variables|Default|GetTargetOffset)))) (.z (Transformation|GetActorLocation)))))
              (Rendering|Material|SetScalarParameterValueonMaterials (Variables|Default|GetSM_turret1_gun) "EmissiveMP" (.x (Math|Interpolation|VInterpTo (Variables|Default|GetMaterialLerp) "14.000000, 0, 0" (Utilities|Time|GetWorldDeltaSeconds) 0.02)))
              (Variables|Default|SetMaterialLerp (Math|Conversions|ToVector(Float) (.x (Math|Interpolation|VInterpTo (Variables|Default|GetMaterialLerp) "14.000000, 0, 0" (Utilities|Time|GetWorldDeltaSeconds) 0.02))))
              (Transformation|SetRelativeRotation (Variables|Default|GetSM_turret1_base) (Math|Interpolation|RInterpTo (Transformation|GetWorldRotation (Variables|Default|GetSM_turret1_base)) (Math|Rotator|MakeRotator (select _downturret 1.8e+02 0.0) 0.0 (+ (.yaw (Math|Rotator|FindLookatRotation (Transformation|GetActorLocation) (Transformation|GetActorLocation (Utilities|Array|Get(acopy) (Variables|/Game/UnderSiege/BluePrints/System/BP_USResponseArea.BP_USResponseArea_C|GetUSResponseAreaTargets _usresponsearearef) (Variables|Default|GetTargetOffset))))) (select _downturret 9e+01 -9e+01))) (Utilities|Time|GetWorldDeltaSeconds) (Variables|USControl|GetYawAimSpeed)) false false)
              (Transformation|SetRelativeRotation _sm_turret1_gun (Math|Interpolation|RInterpTo (Variables|/Script/Engine.SceneComponent|GetRelativeRotation _sm_turret1_gun) (Math|Rotator|MakeRotator (* (.pitch (Math|Rotator|FindLookatRotation (Transformation|GetActorLocation) (Transformation|GetActorLocation (Utilities|Array|Get(acopy) (Variables|/Game/UnderSiege/BluePrints/System/BP_USResponseArea.BP_USResponseArea_C|GetUSResponseAreaTargets _usresponsearearef) (Variables|Default|GetTargetOffset))))) (select _downturret 1.0 -1.0)) 0.0 0.0) (Utilities|Time|GetWorldDeltaSeconds) (Variables|USControl|GetPitchAimSpeed)) false false)
              (Utilities|FlowControl|Delay (Variables|USControl|GetFireRate))
              (Components|Animation|PlayAnimation _sm_turret1_gun_2 "/Game/UnderSiege/Animations/Anim_turret1_gun_Anim.Anim_turret1_gun_Anim" false)
              (Components|Timeline|SetPlayRate _sm_turret1_gun_2 (Variables|USControl|GetGunAnimRate))
              (Game|SpawnActorfromClass "/Game/UnderSiege/BluePrints/Bullet/BP_USBullet1.BP_USBullet1_C" (Math|Transform|MakeTransform (Math|Vector|MakeVector (.x _returnvalue) (.y _returnvalue) (+ (.z _returnvalue) 0.0)) (Transformation|GetWorldRotation _sm_turret1_gun_3) "1.000000,1.000000,1.000000") "AlwaysSpawn" 0 0))
            (else
              (if (< (Class|SkeletalMeshComponent|GetPosition _turret1_shield) 0.5)
                (Components|Animation|PlayAnimation _turret1_shield "/Game/UnderSiege/Animations/Anim_turret1_shield_Anim.Anim_turret1_shield_Anim" false)
                (Components|Timeline|SetPlayRate _turret1_shield 1.0))
              (Utilities|FlowControl|Delay (Variables|USControl|GetReadyTime))
              (Variables|Default|SetIsReady true)))
          (else
            (Variables|Default|SetIsAim false)
            (Variables|Default|SetIsReady false)))
        (else
          (Variables|Default|SetTargetOffset (Math|Random|RandomIntegerinRange 0 (- (Utilities|Array|Length (Variables|/Game/UnderSiege/BluePrints/System/BP_USResponseArea.BP_USResponseArea_C|GetUSResponseAreaTargets _usresponsearearef)) 1)))
          (if (Utilities|IsValid (Utilities|Array|Get(acopy) (Variables|/Game/UnderSiege/BluePrints/System/BP_USResponseArea.BP_USResponseArea_C|GetUSResponseAreaTargets _usresponsearearef) (Variables|Default|GetTargetOffset)))
            (Variables|Default|SetIsAim true)
            (elif (> (.x (Variables|Default|GetMaterialLerp)) 0.0)
              (Rendering|Material|SetScalarParameterValueonMaterials (Variables|Default|GetSM_turret1_gun) "EmissiveMP" (.x (Math|Interpolation|VInterpTo (Variables|Default|GetMaterialLerp) "0, 0, 0" (Utilities|Time|GetWorldDeltaSeconds) 0.7)))
              (Variables|Default|SetMaterialLerp (Math|Conversions|ToVector(Float) (.x (Math|Interpolation|VInterpTo (Variables|Default|GetMaterialLerp) "0, 0, 0" (Utilities|Time|GetWorldDeltaSeconds) 0.7))))
              (Components|Animation|PlayAnimation _turret1_shield_2 "/Game/UnderSiege/Animations/Anim_turret1_shield_Anim.Anim_turret1_shield_Anim" false)
              (Components|Animation|SetPosition _turret1_shield_2 1.0 false)
              (Components|Timeline|SetPlayRate _turret1_shield_2 -5.0))))))
    (:else)))

(fn ConstructionScript)