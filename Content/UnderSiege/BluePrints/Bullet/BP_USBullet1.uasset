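; BP_USBullet1 is a turret bullet in UnderSiege that damages enemies on impact.
; Each tick it sweeps its mesh along local Y by Speed, unscaled by delta time, and it self-destructs after AbsLifeTime.
; On hit, actors tagged USEnemyArhetype are cast to BP_USEnemy1 or BP_USEnemy2 to subtract Damage from health directly.
; The bullet then destroys itself, as it does on untagged hits, but survives if both casts fail.
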(event EventBeginPlay
  (Utilities|FlowControl|Delay (Variables|USControl|GetAbsLifeTime))
  (Actor|DestroyActor))

(event Collision|EventHit
  (params (MyComp :type Primitive%20Component%20Object%20Reference) (Other :type Actor%20Object%20Reference) (OtherComp :type Primitive%20Component%20Object%20Reference) (bSelfMoved :type Boolean) (HitLocation :type Vector :default "0, 0, 0") (HitNormal :type Vector :default "0, 0, 0") (NormalImpulse :type Vector :default "0, 0, 0") (Hit :type Hit%20Result%20Structure%20%28by%20ref%29))
  (bind _hitactor (Collision|BreakHitResult Hit))
  (if (Actor|ActorHasTag _hitactor "USEnemyArhetype")
    (bind _asbp_usenemy_1 (Utilities|Casting|CastToBP_USEnemy1 _hitactor)
      (:then
        (Variables|/Game/UnderSiege/BluePrints/Enemy/BP_USEnemy1.BP_USEnemy1_C|SetUSEnemyHealth _asbp_usenemy_1 (- (Variables|/Game/UnderSiege/BluePrints/Enemy/BP_USEnemy1.BP_USEnemy1_C|GetUSEnemyHealth _asbp_usenemy_1) (Variables|USControl|GetDamage)))
        (Actor|DestroyActor))
      (:CastFailed
        (bind _asbp_usenemy_2 (Utilities|Casting|CastToBP_USEnemy2 _hitactor))
        (Variables|/Game/UnderSiege/BluePrints/Enemy/BP_USEnemy2.BP_USEnemy2_C|SetUSEnemyHealth _asbp_usenemy_2 (- (Variables|/Game/UnderSiege/BluePrints/Enemy/BP_USEnemy2.BP_USEnemy2_C|GetUSEnemyHealth _asbp_usenemy_2) (Variables|USControl|GetDamage)))
        (Actor|DestroyActor)))
    (else
      (Actor|DestroyActor))))

(event EventTick
  (params (DeltaSeconds :type Float%20%28single-precision%29))
  (Transformation|AddLocalOffset (Variables|Default|GetSM_bullet_turret1) (Math|Vector|MakeVector 0.0 (Variables|USControl|GetSpeed) 0.0) true false))

(fn ConstructionScript)