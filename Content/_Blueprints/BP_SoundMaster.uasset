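; BP_SoundMaster plays one of four sound cues (Depre, Button, BenScream, Authorized) and visualizes playback as spawned spectrum bars.
; The construction script gathers every AudioElement actor in the level.
; Each sound event binds a duplicated playback-percent handler that converts progress to seconds and samples the shared ConstantRef constant-Q analysis.
; Each band spawns an AudioVisual at the matching element's StartAudio, Z-scaled by band magnitude.
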(event Custom|CustomEvent_2
  (params (PlayingSoundWave :type Sound%20Wave%20Object%20Reference) (PlaybackPercent :type Float%20%28single-precision%29))
  (Variables|Default|SetPlayedTime (* PlaybackPercent (Variables|Default|GetDuration)))
  (for (_array_element _array_index) (Class|ConstantQNRT|GetNormalizedChannelConstantQatTime (Variables|Default|GetConstant_Ref) (Variables|Default|GetPlayedTime))
    (Utilities|IsValid (Utilities|Array|Get(acopy) (Variables|Default|GetAudio%20Elements) _array_index)
      (:Is%20Valid
        (Game|SpawnActorfromClass "/Game/_Blueprints/AudioVisual.AudioVisual_C" (Math|Transform|MakeTransform (Transformation|GetWorldLocation (Variables|/Game/_Blueprints/AudioElement.AudioElement_C|GetStartAudio (Utilities|Array|Get(acopy) (Variables|Default|GetAudio%20Elements) _array_index))) (Transformation|GetActorRotation (Utilities|Array|Get(acopy) (Variables|Default|GetAudio%20Elements) _array_index)) (Math|Vector|MakeVector 0.05 0.05 (* _array_element 1.5))) "AlwaysSpawn" 0 0)
        (Utilities|FlowControl|Delay 1.5)))))

(event Custom|CustomEvent
  (params (PlayingSoundWave :type Sound%20Wave%20Object%20Reference) (PlaybackPercent :type Float%20%28single-precision%29))
  (Variables|Default|SetPlayedTime (* PlaybackPercent (Variables|Default|GetDuration)))
  (for (_array_element _array_index) (Class|ConstantQNRT|GetNormalizedChannelConstantQatTime (Variables|Default|GetConstant_Ref) (Variables|Default|GetPlayedTime))
    (Utilities|IsValid (Utilities|Array|Get(acopy) (Variables|Default|GetAudio%20Elements) _array_index)
      (:Is%20Valid
        (Game|SpawnActorfromClass "/Game/_Blueprints/AudioVisual.AudioVisual_C" (Math|Transform|MakeTransform (Transformation|GetWorldLocation (Variables|/Game/_Blueprints/AudioElement.AudioElement_C|GetStartAudio (Utilities|Array|Get(acopy) (Variables|Default|GetAudio%20Elements) _array_index))) (Transformation|GetActorRotation (Utilities|Array|Get(acopy) (Variables|Default|GetAudio%20Elements) _array_index)) (Math|Vector|MakeVector 0.05 0.05 (* _array_element 1.5))) "AlwaysSpawn" 0 0)
        (Utilities|FlowControl|Delay 1.5)))))

(event Custom|CustomEvent_1
  (params (PlayingSoundWave :type Sound%20Wave%20Object%20Reference) (PlaybackPercent :type Float%20%28single-precision%29))
  (Variables|Default|SetPlayedTime (* PlaybackPercent (Variables|Default|GetDuration)))
  (for (_array_element _array_index) (Class|ConstantQNRT|GetNormalizedChannelConstantQatTime (Variables|Default|GetConstant_Ref) (Variables|Default|GetPlayedTime))
    (Utilities|IsValid (Utilities|Array|Get(acopy) (Variables|Default|GetAudio%20Elements) _array_index)
      (:Is%20Valid
        (Game|SpawnActorfromClass "/Game/_Blueprints/AudioVisual.AudioVisual_C" (Math|Transform|MakeTransform (Transformation|GetWorldLocation (Variables|/Game/_Blueprints/AudioElement.AudioElement_C|GetStartAudio (Utilities|Array|Get(acopy) (Variables|Default|GetAudio%20Elements) _array_index))) (Transformation|GetActorRotation (Utilities|Array|Get(acopy) (Variables|Default|GetAudio%20Elements) _array_index)) (Math|Vector|MakeVector 0.05 0.05 (* _array_element 1.5))) "AlwaysSpawn" 0 0)
        (Utilities|FlowControl|Delay 1.5)))))

(event Custom|CustomEvent_3
  (params (PlayingSoundWave :type Sound%20Wave%20Object%20Reference) (PlaybackPercent :type Float%20%28single-precision%29))
  (Variables|Default|SetPlayedTime (* PlaybackPercent (Variables|Default|GetDuration)))
  (for (_array_element _array_index) (Class|ConstantQNRT|GetNormalizedChannelConstantQatTime (Variables|Default|GetConstant_Ref) (Variables|Default|GetPlayedTime))
    (Utilities|IsValid (Utilities|Array|Get(acopy) (Variables|Default|GetAudio%20Elements) _array_index)
      (:Is%20Valid
        (Game|SpawnActorfromClass "/Game/_Blueprints/AudioVisual.AudioVisual_C" (Math|Transform|MakeTransform (Transformation|GetWorldLocation (Variables|/Game/_Blueprints/AudioElement.AudioElement_C|GetStartAudio (Utilities|Array|Get(acopy) (Variables|Default|GetAudio%20Elements) _array_index))) (Transformation|GetActorRotation (Utilities|Array|Get(acopy) (Variables|Default|GetAudio%20Elements) _array_index)) (Math|Vector|MakeVector 0.05 0.05 (* _array_element 1.5))) "AlwaysSpawn" 0 0)
        (Utilities|FlowControl|Delay 1.5)))))

(event EventBenScream
  (bind _scream (Variables|Default|GetScream))
  (Audio|Components|Audio|SetSound (Variables|Default|GetAudio) _scream)
  (Variables|Default|SetDuration (Variables|/Script/Engine.SoundBase|GetDuration _scream))
  (EventDispatchers|BindEventtoOnAudioPlaybackPercent (Variables|Default|GetAudio) (delegate Custom|CustomEvent_1))
  (Audio|Components|Audio|Play (Variables|Default|GetAudio) 0.0))

(event EventAuthorized
  (bind _authorize (Variables|Default|GetAuthorize))
  (Development|PrintString "butt")
  (Audio|Components|Audio|SetSound (Variables|Default|GetAudio) _authorize)
  (Variables|Default|SetDuration (Variables|/Script/Engine.SoundBase|GetDuration _authorize))
  (EventDispatchers|BindEventtoOnAudioPlaybackPercent (Variables|Default|GetAudio) (delegate Custom|CustomEvent_2))
  (Audio|Components|Audio|Play (Variables|Default|GetAudio) 0.0))

(event EventButton
  (Audio|Components|Audio|SetSound (Variables|Default|GetAudio) (Variables|Default|GetButton_0))
  (Variables|Default|SetDuration (Variables|/Script/Engine.SoundBase|GetDuration (Variables|Default|GetButton_0)))
  (EventDispatchers|BindEventtoOnAudioPlaybackPercent (Variables|Default|GetAudio) (delegate Custom|CustomEvent))
  (Audio|Components|Audio|Play (Variables|Default|GetAudio) 0.0))

(event EventDepre
  (Audio|Components|Audio|SetSound (Variables|Default|GetAudio) (Variables|Default|GetDepre_0))
  (Variables|Default|SetDuration (Variables|/Script/Engine.SoundBase|GetDuration (Variables|Default|GetDepre_0)))
  (EventDispatchers|BindEventtoOnAudioPlaybackPercent (Variables|Default|GetAudio) (delegate Custom|CustomEvent_3))
  (Audio|Components|Audio|Play (Variables|Default|GetAudio) 0.0))

(fn ConstructionScript
  (bind _outactors (Actor|GetAllActorsOfClass "/Game/_Blueprints/AudioElement.AudioElement_C"))
  (Variables|Default|SetAudio%20Elements _outactors))