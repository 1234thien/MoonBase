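; Nuke frigate spaceship Blueprint with helper functions for animating doors and firing nuke missiles.
; DoorOpening swings a given door's pitch from closed to a right angle by lerping on an alpha, keeping its roll and yaw.
; Launch casts a Child Actor component's actor to the GB5 frigate missile class and calls its Launch.
; MissileLaunch is an empty stub, and nothing here calls these functions.
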(fn ConstructionScript)