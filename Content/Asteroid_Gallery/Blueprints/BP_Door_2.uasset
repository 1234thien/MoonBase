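; BP_Door_2 is an interactive Asteroid Gallery door that the player opens with the F key while standing nearby.
; Entering the proximity trigger enables input on the actor, and pressing F sets AGPlayerNear on the door mesh's ABP_AG_Door animation blueprint.
; Leaving the trigger disables input and clears the flag, leaving the door motion to the animation blueprint.
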(event OnComponentEndOverlap(Door_Proximity)
  (params (OverlappedComponent :type Primitive%20Component%20Object%20Reference) (OtherActor :type Actor%20Object%20Reference) (OtherComp :type Primitive%20Component%20Object%20Reference) (OtherBodyIndex :type Integer))
  (Input|DisableInput (Game|GetPlayerController 0))
  (bind _asabp_ag_door (Utilities|Casting|CastToABP_AG_Door (Components|SkeletalMesh|GetAnimInstance (Variables|Default|GetSM_Door))))
  (Variables|/Game/Asteroid_Gallery/Meshes/AG_Door/ABP_AG_Door.ABP_AG_Door_C|SetAG_Player_near _asabp_ag_door false))

(event OnComponentBeginOverlap(Door_Proximity)
  (params (OverlappedComponent :type Primitive%20Component%20Object%20Reference) (OtherActor :type Actor%20Object%20Reference) (OtherComp :type Primitive%20Component%20Object%20Reference) (OtherBodyIndex :type Integer) (bFromSweep :type Boolean) (SweepResult :type Hit%20Result%20Structure%20%28by%20ref%29))
  (Input|EnableInput (Game|GetPlayerController 0)))

(event Input|KeyboardEvents|F
  (params (Key :type Key%20Structure))
  (:Pressed
    (if true
      (bind _asabp_ag_door (Utilities|Casting|CastToABP_AG_Door (Components|SkeletalMesh|GetAnimInstance (Variables|Default|GetSM_Door))))
      (Variables|/Game/Asteroid_Gallery/Meshes/AG_Door/ABP_AG_Door.ABP_AG_Door_C|SetAG_Player_near _asabp_ag_door true))))

(fn ConstructionScript)